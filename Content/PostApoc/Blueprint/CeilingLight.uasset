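; Ceiling light fixture Blueprint that pairs a static mesh with a spot light, configured entirely in the construction script.
; It creates a dynamic material instance from the ceiling light material and uses a toggle to switch the fixture on or off.
; A single strength value drives both the material's emissive glow and the scaled spot light intensity, zeroing both when off.
; The event graph has no active logic.
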(fn `UserConstructionScript`
  (bind _dmi (`self.DMI`))
  (bind _lightstrength (`self.LightStrength`))
  (bind _spotlight (`self.SpotLight`))
  (bind _returnvalue (`PrimitiveComponent.CreateDynamicMaterialInstance` (`self.StaticMesh`) 0 "/Game/PostApoc/Materials/CeilingLight_mat.CeilingLight_mat"))
  (set `self.DMI` _returnvalue)
  (if (`self.Light Toggle `)
    (`MaterialInstanceDynamic.SetScalarParameterValue` _dmi "Emissive Strength" _lightstrength)
    (`LightComponent.SetIntensity` _spotlight (* _lightstrength 1000.0))
    (else
      (`MaterialInstanceDynamic.SetScalarParameterValue` _dmi "Emissive Strength" 0.0)
      (`LightComponent.SetIntensity` _spotlight 0.0))))